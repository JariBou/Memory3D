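; BP_Card is a flippable card in a memory pair-matching game, showing an image texture or, failing that, its PairID as text.
; Interact asks GM_Memory whether flipping is allowed, then FlipCard alternates a Timeline forward and backward to move and roll the cube.
; The face is revealed as the forward flip starts and hidden when the reverse ends.
; The card reserves a spot on reveal and notifies the game mode after each flip.
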(event `self.ReceiveBeginPlay`
  (bind _imagetexture (`self.ImageTexture`))
  (bind _returnvalue (`KismetTextLibrary.Conv_IntToText` (`self.PairID`)))
  (set `self.CubeRelativeStartingPosition` (`SceneComponent.RelativeLocation` (`self.Cube`)))
  (bind _asgm_memory (cast `/Game/_project/BP/GM_Memory` (`GameplayStatics.GetGameMode`)))
  (set `self.GameMode` _asgm_memory)
  (`TextRenderComponent.K2_SetText` (`self.PairIDDebug`) _returnvalue)
  (`TextRenderComponent.K2_SetText` (`self.FallbackIdDisplay`) _returnvalue)
  (bind _returnvalue_2 (`|CreateWidget` "/Game/_project/Widgets/WD_CardImageDisplay.WD_CardImageDisplay_C"))
  (`WidgetComponent.SetWidget` (`self.ImageDisplay`) _returnvalue_2)
  (`/Engine/EditorBlueprintResources/StandardMacros.IsValid` _imagetexture
    (:`Is Valid`
      (`Image.SetBrushFromTexture` (`/Game/_project/Widgets/WD_CardImageDisplay.Image_41` _returnvalue_2) _imagetexture false)
      (set `self.HasTexture` true))
    (:`Is Not Valid`
      _))
  (`self.SetDisplayState` false))

(event `FlipCard`
  (set `self.IsFlipping` true)
  (bind _isa (`/Engine/EditorBlueprintResources/StandardMacros.FlipFlop`)
    (:`A`
      (`/Game/_project/BP/GM_Memory.ReserveSpot` (`self.GameMode`))
      (`self.SetDisplayState` true)
      (set `self.Flipped` true)
      (bind (_direction _positioncurve _rotationcurve) (`Timeline|Timeline` :!via `PlayFromStart` :!label _label)
        (:`Update`
          (`SceneComponent.K2_SetRelativeLocationAndRotation` (`self.Cube`) (+ (`self.CubeRelativeStartingPosition`) _positioncurve) (`KismetMathLibrary.MakeRotator` (.x _rotationcurve)) false false))
        (:`Finished`
          (bind _returnvalue (not _isa))
          (if _returnvalue
            (`self.SetDisplayState` false))
          (set `self.IsFlipping` false)
          (`/Game/_project/BP/GM_Memory.NotifyCardFlipped` (`self.GameMode`) _returnvalue self))))
    (:`B`
      (set `self.Flipped` false)
      (goto _label :!via `ReverseFromEnd`))))

(event `/Game/_project/BP/Interfaces/IN_Interactable.Interact`
  (bind _canflip (`/Game/_project/BP/GM_Memory.CanFlipCard` (`self.GameMode`)))
  (if (and _canflip (and (not (`self.IsFlipping`)) (`self.IsEnabled`)))
    (set `self.IsFlipping` true)
    (`self.FlipCard`)))

(event `DisableCard`
  (set `self.IsEnabled` false))

(fn `SetDisplayState`
  (params (State :type Boolean))
  (if (`self.HasTexture`)
    (`SceneComponent.SetVisibility` (`self.ImageDisplay`) State false)
    (else
      (`SceneComponent.SetVisibility` (`self.FallbackIdDisplay`) State false))))

(fn `UserConstructionScript`)
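; Card spawner for a memory game that, on BeginPlay, hides the cursor, sets game-only input and lays out a grid of BP_Card actors.
; The game instance's pair count yields a shuffled list of duplicated pair IDs, dealt one per card with its image from DAT_PairImageInfo.
; FindGridSize seeks a near-square grid using the largest divisor up to the square root, and each card's bounds set the spacing.
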(event `self.ReceiveBeginPlay`
  (bind _returnvalue (`GameplayStatics.GetPlayerController` 0))
  (bind _possiblepairids (`self.PossiblePairIDs`))
  (bind (_x _y) (`self.FindGridSize` (* (`/Game/_project/BP/BP_MemoryGameInstance.NumberOfPairs` (`self.GameInstance`)) 2)))
  (bind _asbp_memory_game_instance (cast `/Game/_project/BP/BP_MemoryGameInstance` (`GameplayStatics.GetGameInstance`)))
  (set `self.GameInstance` _asbp_memory_game_instance)
  (set `PlayerController.bShowMouseCursor` false _returnvalue)
  (`WidgetBlueprintLibrary.SetInputMode_GameOnly` _returnvalue)
  (for _index (range (`/Game/_project/BP/BP_MemoryGameInstance.NumberOfPairs` (`self.GameInstance`)))
    (bind _returnvalue_2 (`|Copy` _index))
    (`KismetArrayLibrary.Array_Add` _possiblepairids _returnvalue_2)
    (`KismetArrayLibrary.Array_Add` _possiblepairids _returnvalue_2))
  (`KismetArrayLibrary.Array_Shuffle` _possiblepairids)
  (for _ (range (+ _x 1))
    (set `self.Prev X` 0.0)
    (for _ (range (+ _y 1))
      (bind _output (`self.GeneratePairId`))
      (bind _image (`self.GetCardPairImage` _output))
      (bind _returnvalue_3 (`|SpawnActorFromClass` "/Game/_project/BP/BP_Card.BP_Card_C" (`KismetMathLibrary.MakeTransform` (`KismetMathLibrary.MakeVector` (`self.Prev X`) (`self.prevY`))) "Undefined" "MultiplyWithRoot" null _output _image null))
      (bind (_origin _boxextent) (`self.GetActorBounds` _returnvalue_3 false false))
      (set `self.Prev X` (+ (* (.x _boxextent) 2.3) (`self.Prev X`))))
    (set `self.prevY` (+ (* (.y _boxextent) 2.3) (`self.prevY`)))))

(fn `FindGridSize`
  (params (NumberOfCards :type Integer))
  (returns (X :type Integer) (Y :type Integer))
  (locals (LastDivisor :type Integer))
  (bind _numberofcards (`local.NumberOfCards`))
  (bind _lastdivisor (`local.LastDivisor`))
  (for _index (range 2 (+ (`KismetMathLibrary.FTrunc` (`KismetMathLibrary.Sqrt` (`KismetMathLibrary.Conv_IntToDouble` NumberOfCards))) 1))
    (bind (_remainder _returnvalue) (`KismetMathLibrary.FMod` (`KismetMathLibrary.Conv_IntToDouble` _numberofcards) (`KismetMathLibrary.Conv_IntToDouble` _index)))
    (if (== _remainder 0.0)
      (set `local.LastDivisor` _returnvalue)))
  (return (- (/ _numberofcards _lastdivisor) 1) (- _lastdivisor 1)))

(fn `GeneratePairId`
  (returns (Output :type Integer))
  (locals (TempId :type Integer))
  (set `local.TempId` (`|GetArrayItem` (`self.PossiblePairIDs`)))
  (`KismetArrayLibrary.Array_Remove` (`self.PossiblePairIDs`))
  (return (`local.TempId`)))

(fn `GetCardPairImage`
  (params (PairID :type Integer))
  (returns (Image :type "Texture2D Object Reference"))
  (bind _returnvalue (`|GetDataTableRow` "/Game/_project/DataAssets/DAT_PairImageInfo.DAT_PairImageInfo" (`KismetStringLibrary.Conv_StringToName` (`KismetStringLibrary.Conv_IntToString` PairID)))
    (:`then`
      (return (break `/Game/_project/DataAssets/ST_PairImageInfo` _returnvalue)))
    (:`RowNotFound`
      (return null))))

(fn `UserConstructionScript`)
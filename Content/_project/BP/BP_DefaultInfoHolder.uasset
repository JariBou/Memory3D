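; BP_DefaultInfoHolder is an actor that supplies default difficulty data to the memory game and brings up the main menu.
; On BeginPlay it passes its DifficultyInfoMap to BP_MemoryGameInstance through Instantiate and sets the initial selected difficulty.
; It then creates the WD_MainMenu widget, shows the mouse cursor and switches input to UI only with the menu focused.
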(event `self.ReceiveBeginPlay`
  (bind _returnvalue (`GameplayStatics.GetPlayerController` 0))
  (bind _asbp_memory_game_instance (cast `/Game/_project/BP/BP_MemoryGameInstance` (`GameplayStatics.GetGameInstance`)))
  (bind _output_get (set `self.GameInstance` _asbp_memory_game_instance))
  (`/Game/_project/BP/BP_MemoryGameInstance.Instantiate` _output_get (`self.DifficultyInfoMap`))
  (set `/Game/_project/BP/BP_MemoryGameInstance.SelectedDifficulty` "NewEnumerator0" (`self.GameInstance`))
  (bind _returnvalue_2 (`|CreateWidget` "/Game/_project/Widgets/WD_MainMenu.WD_MainMenu_C"))
  (`UserWidget.AddToViewport` _returnvalue_2 0)
  (set `PlayerController.bShowMouseCursor` true _returnvalue)
  (`WidgetBlueprintLibrary.SetInputMode_UIOnlyEx` _returnvalue _returnvalue_2))

(fn `UserConstructionScript`)
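; Game instance for a memory game that holds the selected difficulty and its settings across the session.
; Instantiate copies a base difficulty map into a working map and a default-values map, and GetDifficultyInfo returns the working entry for the selection.
; ResetDifficulty restores that entry from the defaults.
; NewGame sets the difficulty and iterates the passed map's keys, but rewrites the working map's own values, ignoring the passed ones.
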(fn `GetDifficultyInfo`
  (returns (Info :type "/Game/_project/BP/Structures/ST_DifficultyInfo Structure"))
  (return (`BlueprintMapLibrary.Map_Find` (`self.DifficultyInfoMap`) (`self.SelectedDifficulty`))))

(fn `Instantiate`
  (params (BaseDifficultyMap :type "Map of /Game/_project/BP/Enums/EN_Difficulty Enum to /Game/_project/BP/Structures/ST_DifficultyInfo Structure"))
  (bind _keys (`BlueprintMapLibrary.Map_Keys` BaseDifficultyMap))
  (for _array_element _keys
    (bind _value (`BlueprintMapLibrary.Map_Find` (`local.BaseDifficultyMap`) _array_element))
    (`BlueprintMapLibrary.Map_Add` (`self.DifficultyInfoMap`) _array_element _value)
    (`BlueprintMapLibrary.Map_Add` (`self.DifficultyInfoMap_DefaultValues`) _array_element _value)))

(fn `NewGame`
  (params (`New Map` :type "Map of /Game/_project/BP/Enums/EN_Difficulty Enum to /Game/_project/BP/Structures/ST_DifficultyInfo Structure") (DifficultyLevel :type "/Game/_project/BP/Enums/EN_Difficulty Enum" :default "NewEnumerator0"))
  (set `self.SelectedDifficulty` DifficultyLevel)
  (bind _keys (`BlueprintMapLibrary.Map_Keys` `New Map`))
  (for _array_element _keys
    (`BlueprintMapLibrary.Map_Add` (`self.DifficultyInfoMap`) _array_element (`BlueprintMapLibrary.Map_Find` (`self.DifficultyInfoMap`) _array_element))))

(fn `ResetDifficulty`
  (bind _selecteddifficulty (`self.SelectedDifficulty`))
  (`BlueprintMapLibrary.Map_Add` (`self.DifficultyInfoMap`) _selecteddifficulty (`BlueprintMapLibrary.Map_Find` (`self.DifficultyInfoMap_DefaultValues`) _selecteddifficulty)))
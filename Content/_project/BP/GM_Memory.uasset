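; Game mode for a memory card-matching game that tracks flipped cards and elapsed play time.
; Flip notifications fill a list; at two cards it compares pair IDs, disabling a match or flipping both back.
; A reserved-spot counter limits flips to two at once and drops when a card resets or a pair resolves.
; Tick accumulates the timer and pushes it to the HUD cached at BeginPlay.
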(event `self.ReceiveBeginPlay`
  (bind _aswbp_hud (cast `/Game/_project/Widgets/WBP_HUD` (`PlayerController.GetHUD` (`GameplayStatics.GetPlayerController` 0))))
  (set `self.WBPHud` _aswbp_hud))

(event `self.ReceiveTick`
  (params (DeltaSeconds :type "Float (single-precision)"))
  (bind _output_get (set `self._timer` (+ DeltaSeconds (`self._timer`))))
  (`/Game/_project/Widgets/WD_MainHud.UpdateTimer` (`/Game/_project/Widgets/WBP_HUD.MainHud` (`self.WBPHud`)) _output_get))

(event `NotifyCardFlipped`
  (params (IsReset :type Boolean) (FlippedCard :type "/Game/_project/BP/BP_Card Object Reference"))
  (bind _flippedcards (`self.FlippedCards`))
  (if (not IsReset)
    (`KismetArrayLibrary.Array_Add` _flippedcards FlippedCard)
    (if (== (`KismetArrayLibrary.Array_Length` _flippedcards) 2)
      (`self.TestValidPair`))
    (else
      (`KismetArrayLibrary.Array_RemoveItem` _flippedcards FlippedCard)
      (set `self.ReservedSpots` (- (`self.ReservedSpots`) 1)))))

(event `ReserveSpot`
  (set `self.ReservedSpots` (+ (`self.ReservedSpots`) 1)))

(fn `CanFlipCard`
  (returns (CanFlip :type Boolean))
  (return (< (`self.ReservedSpots`) 2)))

(fn `IsFlippedCardsPair`
  (returns (IsPair :type Boolean))
  (bind _flippedcards (`self.FlippedCards`))
  (return (== (`/Game/_project/BP/BP_Card.PairID` (`|GetArrayItem` _flippedcards)) (`/Game/_project/BP/BP_Card.PairID` (`|GetArrayItem` _flippedcards 1)))))

(fn `ReserveSpotFunc`
  (set `self.ReservedSpots` (+ (`self.ReservedSpots`) 1)))

(fn `TestValidPair`
  (bind _flippedcards (`self.FlippedCards`))
  (bind _ispair (`self.IsFlippedCardsPair`))
  (for _array_element _flippedcards
    (if _ispair
      (`/Game/_project/BP/BP_Card.DisableCard` _array_element)
      (else
        (`/Game/_project/BP/BP_Card.FlipCard` _array_element))))
  (`KismetArrayLibrary.Array_Clear` _flippedcards)
  (set `self.ReservedSpots` 0))

(fn `UserConstructionScript`)